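; Blueprint function library of typed getters for core gameplay objects.
; It returns the game mode cast to BP_GameMode, the first player controller cast to BP_PlayerController, and a given controller's controlled pawn cast to Character.
; Each getter prints an error string when its cast fails.
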(fn GetGameModeBP
  (bind _asbp_game_mode (Utilities|Casting|CastToBP_GameMode (Game|GetGameMode))
    (:then
      _)
    (:CastFailed
      (Development|PrintString 0 "Unable to find GameMode")))
  (return _asbp_game_mode))

(fn GetPlayerControllerBP
  (bind _asbp_player_controller (Utilities|Casting|CastToBP_PlayerController (Game|GetPlayerController 0))
    (:then
      _)
    (:CastFailed
      (Development|PrintString 0 "Failed to get PlayerController")))
  (return _asbp_player_controller))

(fn GetCharacterBP
  (params (Target :type Controller%20Object%20Reference))
  (bind _ascharacter (Utilities|Casting|CastToCharacter (Pawn|GetControlledPawn Target))
    (:then
      _)
    (:CastFailed
      (Development|PrintString 0 "Failed to get ControlledPawn as Character")))
  (return _ascharacter))