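; Player controller Blueprint that possesses a character and drives its movement and jumping.
; An Init event takes the character, possesses it and enables input.
; Every tick, Move feeds the controlled pawn movement input along a Direction variable, which nothing in these graphs sets, scaled by delta seconds.
; The Jump action calls Jump through a helper that casts the pawn to Character and prints a message on failure.
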(event Custom|Init
  (params (playerCharacter_BP :type BP%20Player%20Character%20Object%20Reference))
  ;[1 1 1] Init
  (Pawn|Possess playerCharacter_BP)
  (Input|EnableInput 0))

(event EventTick
  (params (DeltaSeconds :type Float%20%28single-precision%29))
  ;[1 1 1] Move
  (CallFunction|Move (Variables|Default|Getdirection) DeltaSeconds))

(event Input|ActionEvents|InputActionJump
  (params (Key :type Key%20Structure :default "AnyKey"))
  ;[1 1 1] Move
  (:Pressed
    (bind _ascharacter (CallFunction|GetCharacterBP self))
    (Character|Jump _ascharacter)))

(fn ConstructionScript)

(fn GetCharacterBP
  (bind _ascharacter (Utilities|Casting|CastToCharacter (Pawn|GetControlledPawn))
    (:then
      _)
    (:CastFailed
      (Development|PrintString "Failed to get ControlledPawn as Character")))
  (return _ascharacter))

(fn Move
  (params (direction :type Vector) (axisValue :type Float%20%28single-precision%29))
  (Pawn|Input|AddMovementInput (Pawn|GetControlledPawn) direction axisValue false)
  (return))